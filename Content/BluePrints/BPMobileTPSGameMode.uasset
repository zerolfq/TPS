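; Game mode for a mobile third-person shooter that handles kill scoring and guard bot spawning.
; On BeginPlay it binds to the actor-killed event, awarding the killer's MobileTPSPlayerState points when the victim is a pawn other than a ThirdPersonCharacter.
; SpawnNewBot, not called within this graph, runs the EQ_Guard EQS query and spawns a BPAIGuard at each returned location, adjusting for collisions.
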(event `self.ReceiveBeginPlay`
  (add `self.OnActorKilled` (delegate `HandleOnActorKilled`)))

(event `HandleOnActorKilled` :!signature `self.OnActorKilled`
  (params (VictimActor :type "Actor Object Reference") (KillerActor :type "Actor Object Reference") (KillerController :type "Controller Object Reference"))
  (bind _aspawn (cast `Pawn` VictimActor))
  (cast `/Game/BluePrints/ThirdPersonCharacter` _aspawn
    (:`CastFailed`
      (bind _asmobile_tpsplayer_state (cast `MobileTPSPlayerState` (`Pawn.PlayerState` (`Controller.K2_GetPawn` KillerController))))
      (`MobileTPSPlayerState.AddScore` _asmobile_tpsplayer_state 20.0))))

(event `self.SpawnNewBot`
  (bind _returnvalue (`EnvQueryManager.RunEQSQuery` "/Game/Behavior/EQ_Guard.EQ_Guard" self "RandomBest25Pct"))
  (add `EnvQueryInstanceBlueprintWrapper.OnQueryFinishedEvent` _returnvalue (delegate `OnQueryFinishedEvent_Event`)))

(event `OnQueryFinishedEvent_Event`
  (params (QueryInstance :type "EnvQueryInstanceBlueprintWrapper Object Reference") (QueryStatus :type "EEnvQueryStatus Enum" :default "Processing"))
  (switch `EEnvQueryStatus` QueryStatus
    (:`Success`
      (bind _resultlocations (`EnvQueryInstanceBlueprintWrapper.GetQueryResultsAsLocations` QueryInstance))
      (for _array_element _resultlocations
        (`|SpawnActorFromClass` "/Game/BluePrints/BPAIGuard.BPAIGuard_C" (`KismetMathLibrary.MakeTransform` _array_element) "AdjustIfPossibleButDontSpawnIfColliding" "OverrideRootScale" null null)))))

(fn `UserConstructionScript`)